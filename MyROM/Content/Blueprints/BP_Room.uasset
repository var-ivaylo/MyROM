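; BP_Room is a configurable showcase room with a door, an interactable item, game info text and three picture walls.
; Its construction script applies the texts and item class and creates transparent dynamic materials for text and pictures.
; Overlapping the item's trigger enables actor input, and Interact works once, unbinding the trigger while a timeline shrinks the item's effect and animates text and picture opacity.
; It also relays the child door's closed event through its own dispatcher.
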(event Custom|OnItemTriggerBeginOverlap
  (params (OtherActor :type Actor%20Object%20Reference) (OtherComp :type Primitive%20Component%20Object%20Reference) (OtherBodyIndex :type Integer) (bFromSweep :type Boolean) (SweepResult :type Hit%20Result%20Structure%20%28by%20ref%29))
  (Input|EnableInput (Game|GetPlayerController 0)))

(event Custom|OnItemTriggerEndOverlap
  (params (OtherActor :type Actor%20Object%20Reference) (OtherComp :type Primitive%20Component%20Object%20Reference) (OtherBodyIndex :type Integer))
  (Input|DisableInput (Game|GetPlayerController 0)))

(event Custom|OnDoorClosed_Event
  (Default|CallOnDoorClosed))

(event EventBeginPlay
  (bind _itemref (Variables|Default|GetItemRef))
  (bind _trigger (Variables|/Game/Items/BP_Item.BP_Item_C|GetTrigger _itemref))
  (Utilities|FlowControl|Sequence
    (:then_0
      (bind _asbp_door (Utilities|Casting|CastToBP_Door (Variables|/Script/Engine.ChildActorComponent|GetChildActor (Variables|Default|GetBP_Door))))
      (EventDispatchers|BindEventtoOnDoorClosed _asbp_door (delegate Custom|OnDoorClosed_Event)))
    (:then_1
      (Collision|AssignOnComponentBeginOverlap _trigger (delegate Custom|OnItemTriggerBeginOverlap))
      (Collision|BindEventtoOnComponentEndOverlap _trigger (delegate Custom|OnItemTriggerEndOverlap)))))

(event Input|ActionEvents|InputActionInteract
  (params (Key :type Key%20Structure :default "AnyKey"))
  (bind _itemref (Variables|Default|GetItemRef))
  (bind _trigger (Variables|/Game/Items/BP_Item.BP_Item_C|GetTrigger _itemref))
  (:Pressed
    (Input|DisableInput (Game|GetPlayerController 0))
    (Actor|Tick|SetActorTickEnabled _itemref)
    (Utilities|FlowControl|Sequence
      (:then_0
        (EventDispatchers|UnbindallEventsfromOnComponentBeginOverlap _trigger))
      (:then_1
        (EventDispatchers|UnbindallEventsfromOnComponentEndOverlap _trigger)
        (Development|SetHiddeninGame (Variables|/Game/Items/BP_Item.BP_Item_C|GetInteractText (Variables|Default|GetItemRef)) true true)
        (Development|SetHiddeninGame (Variables|Default|GetGameInfo) false true)
        (bind (_direction _scale _alpha) (Timeline|HideItemAdds PlayFromStart)
          (:Update
            (Utilities|FlowControl|Sequence
              (:then_0
                (bind _returnvalue (Rendering|Material|GetScalarParameterValue (Variables|Default|GetGameInfoTextMaterial) "Opacity" :!class /Script/Engine.MaterialInstanceDynamic))
                (Rendering|Material|SetScalarParameterValue (Variables|Default|GetGameInfoTextMaterial) "Opacity" (Class|KismetMathLibrary|InverseLerp _returnvalue 1.0 _alpha) :!class /Script/Engine.MaterialInstanceDynamic))
              (:then_1
                (Transformation|SetWorldScale3D (Variables|/Game/Items/BP_Item.BP_Item_C|GetEffect (Variables|Default|GetItemRef)) (Math|Vector|Lerp(Vector) (Transformation|GetWorldScale (Variables|/Game/Items/BP_Item.BP_Item_C|GetEffect (Variables|Default|GetItemRef))) "0,0.000000, 0" _scale)))
              (:then_2
                (Development|SetHiddeninGame (Variables|Default|GetPictures) false true)
                (for _array_element (Variables|Default|GetPicturesDynamicMats)
                  (bind _returnvalue_2 (Rendering|Material|GetScalarParameterValue _array_element "Opacity" :!class /Script/Engine.MaterialInstanceDynamic))
                  (Rendering|Material|SetScalarParameterValue _array_element "Opacity" (Class|KismetMathLibrary|InverseLerp _returnvalue_2 1.0 _alpha) :!class /Script/Engine.MaterialInstanceDynamic)))))
          (:Finished
            (Development|SetHiddeninGame (Variables|/Game/Items/BP_Item.BP_Item_C|GetEffect (Variables|Default|GetItemRef)) true true)
            (Development|SetHiddeninGame (Variables|/Game/Items/BP_Item.BP_Item_C|GetInteractText (Variables|Default|GetItemRef)) true true)))))))

(fn ConstructionScript
  (Rendering|Components|TextRender|SetText (Variables|Default|GetGameInfo) (Variables|RoomInfo|GetGameInfoText))
  (bind _returnvalue (Rendering|Material|CreateDynamicMaterialInstance (Variables|Default|GetGameInfo) 0 "/Game/Meshes/Materials/TextEmissionMaterial.TextEmissionMaterial" :!class /Script/Engine.PrimitiveComponent))
  (bind _output_get (Variables|Default|SetGameInfoTextMaterial _returnvalue))
  (Rendering|Material|SetScalarParameterValue _returnvalue "Opacity" 0.0 :!class /Script/Engine.MaterialInstanceDynamic)
  (Rendering|Material|SetVectorParameterValue _returnvalue "Glow Color" "(R=1.000000,G=1.000000,B=1.000000,A=1.000000)" :!class /Script/Engine.MaterialInstanceDynamic)
  (bind _asbp_door (Utilities|Casting|CastToBP_Door (Variables|/Script/Engine.ChildActorComponent|GetChildActor (Variables|Default|GetBP_Door))))
  (Default|SetDoorText _asbp_door (Variables|RoomInfo|GetDoorText))
  (ChildActorComponent|SetChildActorClass (Variables|Default|GetBP_Item) (Variables|RoomInfo|GetItem))
  (bind _asbp_item (Utilities|Casting|CastToBP_Item (Variables|/Script/Engine.ChildActorComponent|GetChildActor (Variables|Default|GetBP_Item))))
  (Variables|Default|SetItemRef _asbp_item)
  (bind _returnvalue_2 (Rendering|Material|CreateDynamicMaterialInstance (Variables|Default|GetMainPicWall) 0 (Variables|Pictures|GetMainPicMaterial) :!class /Script/Engine.PrimitiveComponent))
  (Utilities|Array|Add (Variables|Default|GetPicturesDynamicMats) _returnvalue_2)
  (bind _returnvalue_3 (Rendering|Material|CreateDynamicMaterialInstance (Variables|Default|GetLeftPicWall) 0 (Variables|Pictures|GetLeftPicMaterial) :!class /Script/Engine.PrimitiveComponent))
  (Utilities|Array|Add (Variables|Default|GetPicturesDynamicMats) _returnvalue_3)
  (bind _returnvalue_4 (Rendering|Material|CreateDynamicMaterialInstance (Variables|Default|GetRightPicWall) 0 (Variables|Pictures|GetRightPicMaterial) :!class /Script/Engine.PrimitiveComponent))
  (Utilities|Array|Add (Variables|Default|GetPicturesDynamicMats) _returnvalue_4)
  (for _array_element (Variables|Default|GetPicturesDynamicMats)
    (Rendering|Material|SetScalarParameterValue _array_element "Opacity" 0.0 :!class /Script/Engine.MaterialInstanceDynamic)))