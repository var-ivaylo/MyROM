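; One-way door Blueprint that swings open the first time something overlaps EnterBox, then shuts on a LeaveBox overlap and shows a red X.
; Timelines lerp rotation and emission from current values, dimming door and number glow on opening and brightening the X on closing.
; DoorLocked is set on opening and never cleared here, preventing reopening.
; Construction creates the glow material instances, and SetDoorText sets the title.
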(event OnComponentBeginOverlap(EnterBox)
  (params (OtherActor :type Actor%20Object%20Reference) (OtherComp :type Primitive%20Component%20Object%20Reference) (OtherBodyIndex :type Integer) (bFromSweep :type Boolean) (SweepResult :type Hit%20Result%20Structure%20%28by%20ref%29))
  (if (not (Variables|Default|GetDoorLocked))
    (Variables|Default|SetDoorLocked true)
    (bind _rotation (Timeline|OpenDoor PlayFromStart)
      (:Update
        (Transformation|SetRelativeRotation (Variables|Default|GetBlackDoor_Door) (Math|Rotator|Lerp(Rotator) (Variables|/Script/Engine.SceneComponent|GetRelativeRotation (Variables|Default|GetBlackDoor_Door)) (Math|Rotator|MakeRotator 0.0 0.0 9e+01) _rotation true) false false)
        (Utilities|FlowControl|Sequence
          (:then_0
            (bind _returnvalue (Rendering|Material|GetScalarParameterValue (Variables|Default|GetDoorGlower) "Emission Intensity" :!class /Script/Engine.MaterialInstanceDynamic))
            (Rendering|Material|SetScalarParameterValue (Variables|Default|GetDoorGlower) "Emission Intensity" (Math|Float|Lerp _returnvalue 0.0 _rotation) :!class /Script/Engine.MaterialInstanceDynamic))
          (:then_1
            (bind _returnvalue_2 (Rendering|Material|GetScalarParameterValue (Variables|Default|GetDoorNumberGlower) "Emission Intensity" :!class /Script/Engine.MaterialInstanceDynamic))
            (Rendering|Material|SetScalarParameterValue (Variables|Default|GetDoorNumberGlower) "Emission Intensity" (Math|Float|Lerp _returnvalue_2 0.1 _rotation) :!class /Script/Engine.MaterialInstanceDynamic)))))))

(event OnComponentBeginOverlap(LeaveBox)
  (params (OtherActor :type Actor%20Object%20Reference) (OtherComp :type Primitive%20Component%20Object%20Reference) (OtherBodyIndex :type Integer) (bFromSweep :type Boolean) (SweepResult :type Hit%20Result%20Structure%20%28by%20ref%29))
  (Audio|Components|Audio|Stop (Variables|Default|GetOpenDoor))
  (Rendering|Material|SetScalarParameterValue (Variables|Default|GetDoorGlower) "Emission Intensity" 0.0 :!class /Script/Engine.MaterialInstanceDynamic)
  (bind _rotation (Timeline|CloseDoor PlayFromStart)
    (:Update
      (Utilities|FlowControl|Sequence
        (:then_0
          (Transformation|SetRelativeRotation (Variables|Default|GetBlackDoor_Door) (Math|Rotator|Lerp(Rotator) (Variables|/Script/Engine.SceneComponent|GetRelativeRotation (Variables|Default|GetBlackDoor_Door)) "0, 0, 0" _rotation true) false false))
        (:then_1
          (bind _returnvalue (Rendering|Material|GetScalarParameterValue (Variables|Default|GetDoorClosedMarkGlower) "Emission Intensity" :!class /Script/Engine.MaterialInstanceDynamic))
          (Rendering|Material|SetScalarParameterValue (Variables|Default|GetDoorClosedMarkGlower) "Emission Intensity" (Math|Float|Lerp _returnvalue 4.0 _rotation) :!class /Script/Engine.MaterialInstanceDynamic))))))

(fn ConstructionScript
  (bind _doorclosedmark (Variables|Default|GetDoorClosedMark))
  (bind _returnvalue (Rendering|Material|CreateDynamicMaterialInstance (Variables|Default|GetGlower) 0 "/Game/Meshes/Materials/DoorGlowingMaterial.DoorGlowingMaterial" :!class /Script/Engine.PrimitiveComponent))
  (Variables|Default|SetDoorGlower _returnvalue)
  (bind _returnvalue_2 (Rendering|Material|CreateDynamicMaterialInstance (Variables|Default|GetDoorTitleComponent) 0 "/Game/Meshes/Materials/TextGlowingMaterial.TextGlowingMaterial" :!class /Script/Engine.PrimitiveComponent))
  (Variables|Default|SetDoorNumberGlower _returnvalue_2)
  (Rendering|Components|TextRender|SetText _doorclosedmark (Utilities|Text|MakeLiteralText "X"))
  (bind _returnvalue_3 (Rendering|Material|CreateDynamicMaterialInstance _doorclosedmark 0 "/Game/Meshes/Materials/TextGlowingMaterial.TextGlowingMaterial" :!class /Script/Engine.PrimitiveComponent))
  (bind _output_get (Variables|Default|SetDoorClosedMarkGlower _returnvalue_3))
  (Rendering|Material|SetVectorParameterValue _output_get "Glow Color" "(R=1.000000,G=0.000000,B=0.000000,A=1.000000)" :!class /Script/Engine.MaterialInstanceDynamic)
  (Rendering|Material|SetScalarParameterValue _output_get "Emission Intensity" 0.1 :!class /Script/Engine.MaterialInstanceDynamic))

(fn SetDoorText
  (params (DoorNumber :type Text))
  (Rendering|Components|TextRender|SetText (Variables|Default|GetDoorTitleComponent) DoorNumber))