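; BP_Item is an item actor that displays a glowing interaction prompt when something overlaps its trigger.
; Trigger begin and end overlap events show and hide InteractText, without filtering the overlapping actor.
; Every tick the text rotates to face player 0's camera, and the construction script gives it a dynamic material instance with an orange glow.
; The interaction itself is not implemented in these graphs.
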(event OnComponentBeginOverlap(Trigger)
  (params (OtherActor :type Actor%20Object%20Reference) (OtherComp :type Primitive%20Component%20Object%20Reference) (OtherBodyIndex :type Integer) (bFromSweep :type Boolean) (SweepResult :type Hit%20Result%20Structure%20%28by%20ref%29))
  (Development|SetHiddeninGame (Variables|Default|GetInteractText) false true))

(event OnComponentEndOverlap(Trigger)
  (params (OtherActor :type Actor%20Object%20Reference) (OtherComp :type Primitive%20Component%20Object%20Reference) (OtherBodyIndex :type Integer))
  (Development|SetHiddeninGame (Variables|Default|GetInteractText) true true))

(event EventTick
  (params (DeltaSeconds :type Float%20%28single-precision%29))
  (Transformation|SetWorldRotation (Variables|Default|GetInteractText) (Math|Rotator|FindLookatRotation (Transformation|GetWorldLocation (Variables|Default|GetInteractText)) (Transformation|GetActorLocation (Game|GetPlayerCameraManager 0))) false false))

(fn ConstructionScript
  (bind _returnvalue (Rendering|Material|CreateDynamicMaterialInstance (Variables|Default|GetInteractText) 0 "/Game/Meshes/Materials/TextGlowingMaterial.TextGlowingMaterial" :!class /Script/Engine.PrimitiveComponent))
  (Rendering|Material|SetVectorParameterValue _returnvalue "Glow Color" "(R=1.000000,G=0.400000,B=0.000000,A=1.000000)" :!class /Script/Engine.MaterialInstanceDynamic))